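; Base NPC character Blueprint that takes damage, plays a hit reaction and dies as a ragdoll.
; AnyDamage forwards damage to a HealthComponent and plays the punch hit montage.
; The component's OnDeath event turns on mesh physics simulation and disables movement, then a timer destroys the actor a few seconds later.
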(event `self.HealthComponent.OnDeath`
  (`self.Simul and Dis Move`)
  (`KismetSystemLibrary.K2_SetTimerDelegate` (delegate `FinalizeDeath`) 5.0))

(event `FinalizeDeath`
  (`self.K2_DestroyActor`))

(event `self.ReceiveAnyDamage`
  (params (Damage :type "Float (single-precision)") (DamageType :type "DamageType Object Reference") (InstigatedBy :type "Controller Object Reference") (DamageCauser :type "Actor Object Reference"))
  (`/Game/Skvt/Systems/HealthComponent.ProgressDamage` (`self.HealthComponent`) Damage)
  (`self.PlayAnimMontage` "/Game/Skvt/Characters/Animations/Attacks/AM_Hit_punch.AM_Hit_punch"))

(fn `Simul and Dis Move`
  (`PrimitiveComponent.SetSimulatePhysics` (`self.Mesh`) true)
  (`CharacterMovementComponent.DisableMovement` (`self.CharacterMovement`)))

(fn `UserConstructionScript`)