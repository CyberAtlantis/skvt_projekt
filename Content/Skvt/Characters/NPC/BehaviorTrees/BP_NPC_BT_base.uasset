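; Base NPC character Blueprint that can be killed by a stealth assassination from behind.
; The Stealth Back Assasin function plays a neck-break montage, triggers Ragdoll, and returns the AssasinRef world location and the NPC's rotation to the caller.
; Ragdoll waits briefly, enables physics on the mesh, then destroys the actor after a further delay.
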(event `Ragdoll`
  (`KismetSystemLibrary.Delay` 2.5)
  (`PrimitiveComponent.SetSimulatePhysics` (`self.Mesh`) true)
  (`KismetSystemLibrary.Delay` 3.0)
  (`self.K2_DestroyActor`))

(fn `Stealth Back Assasin`
  (returns (RefLocation :type "Vector Structure") (AssasinRotation :type "Rotator Structure"))
  (`self.PlayAnimMontage` "/Game/Skvt/Characters/Animations/Attacks/Hit_BreakNeck_Montage.Hit_BreakNeck_Montage")
  (`self.Ragdoll`)
  (return (`SceneComponent.K2_GetComponentLocation` (`self.Assasin Ref`)) (`self.K2_GetActorRotation`)))

(fn `UserConstructionScript`
  (`parent.UserConstructionScript`))